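; Player controller for the main menu lobby that sets up the lobby UI and relays chat messages.
; On BeginPlay it sets UI-only input and, for the local controller only, creates and stores the WBP_Lobby widget.
; Enter focuses that widget's chatbox, and UpdateChatbox forwards text to GState_Lobby.
; Tick prints a "PC_Lobby" debug string to the screen every frame.
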(event Custom|CreateLobbyWidget
  ;[0 0.7537 0.06764] Create Lobby widget
  (if (Pawn|IsLocalPlayerController)
    (bind _returnvalue (UserInterface|CreateWidget "/Game/MainMenu/WBP_Lobby.WBP_Lobby_C" self))
    (UserInterface|Viewport|AddtoViewport _returnvalue 0)
    (Variables|Default|SetLobbyWidget _returnvalue)))

(event Custom|UpdateChatbox
  (params (InText :type Text))
  ;[0.5894 0 0.2347] Update Chatbox
  (bind _asgstate_lobby (Utilities|Casting|CastToGState_Lobby (Game|GetGameState)))
  (Default|UpdateChatbox _asgstate_lobby InText))

(event EventBeginPlay
  ;[0 0.1932 0.6281] Begin Play
  (Input|SetInputModeUIOnly self 0 "DoNotLock")
  (CallFunction|CreateLobbyWidget))

(event EventTick
  (params (DeltaSeconds :type Float%20%28single-precision%29))
  (Development|PrintString "PC_Lobby" true false "(R=0.000000,G=0.660000,B=1.000000,A=1.000000)" 0.0))

(event Input|KeyboardEvents|Enter
  (params (Key :type Key%20Structure))
  (:Pressed
    (bind _lobbywidget (Variables|Default|GetLobbyWidget)
      (:then
        (Default|FocusChatBox (Variables|/Game/MainMenu/WBP_Lobby.WBP_Lobby_C|GetWBP_Chatbox _lobbywidget)))
      (:else))))

(fn ConstructionScript)