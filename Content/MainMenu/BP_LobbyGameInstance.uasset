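; Lobby game instance that records the class each player selects and initializes global data on startup.
; SelectClass sets the class on the lobby player state, prints the choice, and stores it in an array indexed by PlayerId, growing it as needed.
; GetSelectedClass looks up that array by PlayerId and reports whether the index is valid, so choices can be read independently of the lobby player state.
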(event Custom|SelectClass
  (params (PlayerState :type Player%20State%20Object%20Reference) (Class :type Pawn%20Class%20Reference))
  (bind _playerid (Variables|/Script/Engine.PlayerState|GetPlayerId PlayerState))
  (bind _asplayer_state_lobby (Utilities|Casting|CastToPlayerState_Lobby PlayerState)
    (:then
      (Variables|/Game/MainMenu/PlayerState_Lobby.PlayerState_Lobby_C|SetSelectedClass _asplayer_state_lobby Class)
      (Development|PrintString (Utilities|String|Append "Player " (Utilities|String|ToString(Integer) _playerid) " Selected class " (Utilities|GetClassDisplayName Class)))
      (Utilities|Array|SetArrayElem (Variables|Default|GetLobbySelectedClasses) _playerid Class true))
    (:CastFailed
      (Development|PrintString "Failed to set selected class"))))

(event EventInit
  (|CallParentFunction)
  (Class|FPGAGameplayAbilitiesLibrary|InitGlobalData))

(fn GetSelectedClass
  (params (PlayerState :type Player%20State%20Object%20Reference))
  (bind _playerid (Variables|/Script/Engine.PlayerState|GetPlayerId PlayerState))
  (bind _lobbyselectedclasses (Variables|Default|GetLobbySelectedClasses))
  (bind _returnvalue (Utilities|Array|IsValidIndex _lobbyselectedclasses _playerid))
  (if _returnvalue
    (return (Utilities|Array|Get(acopy) _lobbyselectedclasses _playerid) _returnvalue)
    (else
      (return 0 false))))