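; GA_OnKilled is an event-triggered gameplay ability that handles a unit's death.
; It calls OnKilled on the RTS ability system component, then grants an attribute-based experience reward through a SetByCaller GE_GainExp to the event's OptionalObject actor.
; It plays the death montage from DT_UnitAnimations, sets the owner's lifespan to five seconds and ends immediately, leaving the montage playing.
; The GE_Status_Death application is disconnected.
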(event Custom|ApplyExpReward
  (bind _returnvalue (Ability|GetOwningActorfromActorInfo))
  (bind _returnvalue_2 (Ability|GetAbilitySystemComponent _returnvalue))
  (bind (_bsuccessfullyfoundattribute _returnvalue_3) (Ability|Attribute|GetFloatAttributefromAbilitySystemComponent _returnvalue_2 "(AttributeName=\"ExpReward\",Attribute=StructProperty'\"/Script/OrdersAbilities.RTSProgressionAttributeSet:ExpReward\"',AttributeOwner=Class'\"/Script/OrdersAbilities.RTSProgressionAttributeSet\"')"))
  (if _bsuccessfullyfoundattribute
    (Development|PrintString (Utilities|String|ToString(Float) _returnvalue_3))
    (bind _returnvalue_4 (Ability|GameplayEffect|AssignTagSetbyCallerMagnitude (Ability|MakeOutgoingGameplayEffectSpec "/Game/MyGame/Core/Attributes/Progression/GE_GainExp.GE_GainExp_C") "(TagName=\"SBC.Exp\")" _returnvalue_3))
    (bind _asactor (Utilities|Casting|CastToActor (.OptionalObject (Utilities|Struct|BreakGameplayEventData (Variables|Default|GetCurrentEventData)))))
    (GameplayEffects|ApplyGameplayEffectSpecToTarget _returnvalue_4 (Ability|TargetData|AbilityTargetDatafromActor _asactor))))

(event Ability|EventOnEndAbility
  (params (bWasCancelled :type Boolean)))

(event Ability|EventActivateAbilityFromEvent
  (params (EventData :type Gameplay%20Event%20Data%20Structure%20%28by%20ref%29))
  (bind _returnvalue (Ability|GetOwningActorfromActorInfo))
  (bind _returnvalue_2 (Ability|GetAbilitySystemComponent _returnvalue))
  (bind _asrtsability_system_component (Utilities|Casting|CastToRTSAbilitySystemComponent _returnvalue_2))
  (Development|PrintString "Killed enemy!")
  (Class|RTSAbilitySystemComponent|OnKilled _asrtsability_system_component)
  (CallFunction|ApplyExpReward)
  (Utilities|FlowControl|Sequence
    (:then_0
      (bind _returnvalue_3 (Utilities|GetDataTableRow "/Game/MyGame/Units/DT_UnitAnimations.DT_UnitAnimations" (Class|RTSAbilitySystemComponent|GetName _asrtsability_system_component))
        (:then
          (|PlayMontageandWaitProxy "None" (Utilities|Struct|BreakUnitAnimationRow _returnvalue_3) 1.0 "None" false 1.0))))
    (:then_1
      (Actor|SetLifeSpan (Ability|GetOwningActorfromActorInfo) 5.0)
      (Ability|EndAbility))))