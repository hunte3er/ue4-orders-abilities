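; RTS player controller that creates the game HUD for the local player and forwards unit selection changes to it.
; Hotkeys set pending orders on the RTS controller: attack, or use ability by slot index.
; Debug keys grant experience through a SetByCaller gameplay effect or activate a test ability on selected actors via their ability systems.
; Cursor helpers find ground locations and ability-system actors, but only disconnected debug code calls them.
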(event Custom|ApplyEffectToActors
  (params (GameplayEffectClass :type Gameplay%20Effect%20Class%20Reference))
  (bind _returnvalue (Class|RTSPlayerController|GetSelectedActors))
  (for _array_element _returnvalue
    (bind _returnvalue_2 (Ability|GameplayEffect|AssignTagSetbyCallerMagnitude (GameplayEffects|MakeOutgoingSpec :self (Ability|GetAbilitySystemComponent _array_element) :GameplayEffectClass GameplayEffectClass) "(TagName=\"SBC.Exp\")" 75.0))
    (GameplayEffects|ApplyGameplayEffectSpecToSelf (Ability|GetAbilitySystemComponent _array_element) _returnvalue_2)))

(event EventTick
  (params (DeltaSeconds :type Float%20%28single-precision%29)))

(event EventOnSelectionChanged
  (params (Selection :type Array%20of%20Actor%20Object%20References))
  (Default|OnSelectionChanged (Variables|Default|GetGameUI) Selection))

(event EventBeginPlay
  (Input|SetInputModeGameandUI self 0 "LockAlways" false)
  (Utilities|FlowControl|Sequence
    (:then_1
      (if (Pawn|IsLocalPlayerController)
        (bind _returnvalue (UserInterface|CreateWidget "/Game/MyGame/UI/WBP_GameUI.WBP_GameUI_C"))
        (bind _output_get (Variables|Default|SetGameUI _returnvalue))
        (UserInterface|Viewport|AddtoViewport _output_get 0)))))

(event Input|KeyboardEvents|R
  (params (Key :type Key%20Structure))
  ;[1 0.04688 0] Skill inputs
  (:Pressed
    (Class|RTSPlayerController|SetPendingOrder "/Game/OrdersAbilities/Orders/UseAbilityOrder/BP_UseAbilityOrder.BP_UseAbilityOrder_C" 3)))

(event Input|KeyboardEvents|Z
  (params (Key :type Key%20Structure))
  (:Pressed
    (CallFunction|ApplyEffecttoActors "/Game/MyGame/Test/TestGainExp.TestGainExp_C")))

(event Input|KeyboardEvents|F
  (params (Key :type Key%20Structure))
  ;[1 0.04688 0] Skill inputs
  (:Pressed
    (Class|RTSPlayerController|SetPendingOrder "/Game/OrdersAbilities/Orders/UseAbilityOrder/BP_UseAbilityOrder.BP_UseAbilityOrder_C" 2)))

(event Input|KeyboardEvents|X
  (params (Key :type Key%20Structure))
  (:Pressed
    (bind _returnvalue (Class|RTSPlayerController|GetSelectedActors))
    (for _array_element _returnvalue
      (bind _asrtsability_system_component (Utilities|Casting|CastToRTSAbilitySystemComponent (Ability|GetAbilitySystemComponent _array_element)))
      (Abilities|TryActivateAbilitybyClass _asrtsability_system_component "/Game/MyGame/Test/TestGA.TestGA_C" true))))

(event Input|KeyboardEvents|A
  (params (Key :type Key%20Structure))
  (:Pressed
    (Class|RTSPlayerController|SetPendingOrder "/Game/OrdersAbilities/Orders/AttackOrder/BP_AttackOrder.BP_AttackOrder_C")))

(event Input|KeyboardEvents|Q
  (params (Key :type Key%20Structure))
  ;[1 0.04688 0] Skill inputs
  (:Pressed
    (Class|RTSPlayerController|SetPendingOrder "/Game/OrdersAbilities/Orders/UseAbilityOrder/BP_UseAbilityOrder.BP_UseAbilityOrder_C")))

(event Input|KeyboardEvents|W
  (params (Key :type Key%20Structure))
  ;[1 0.04688 0] Skill inputs
  (:Pressed
    (Class|RTSPlayerController|SetPendingOrder "/Game/OrdersAbilities/Orders/UseAbilityOrder/BP_UseAbilityOrder.BP_UseAbilityOrder_C" 1)))

(event Input|KeyboardEvents|P
  (params (Key :type Key%20Structure))
  ;[1 0.04688 0] Skill inputs
  (:Pressed
    (Class|RTSPlayerController|SetPendingOrder "/Game/OrdersAbilities/Orders/UseAbilityOrder/BP_UseAbilityOrder.BP_UseAbilityOrder_C" 3)))

(event Input|KeyboardEvents|E
  (params (Key :type Key%20Structure))
  ;[1 0.04688 0] Skill inputs
  (:Pressed
    (Class|RTSPlayerController|SetPendingOrder "/Game/OrdersAbilities/Orders/UseAbilityOrder/BP_UseAbilityOrder.BP_UseAbilityOrder_C" 2)))

(fn ConstructionScript)

(fn GetCursorGroundLocation
  (return (.Location (Collision|BreakHitResult (.HitResult (Game|Player|GetHitResultUnderCursorbyChannel "TraceTypeQuery1" true))))))

(fn GetCursorActor
  (bind _array (Utilities|Array|MakeArray "ObjectTypeQuery3" "ObjectTypeQuery2"))
  (bind (_hitresult _returnvalue) (Class|PlayerController|GetHitResultUnderCursorforObjects _array false))
  (bind _hitactor (Collision|BreakHitResult _hitresult))
  (if _returnvalue
    (Utilities|IsValid (Ability|GetAbilitySystemComponent _hitactor)
      (:Is%20Valid
        (return _hitactor))
      (:Is%20Not%20Valid
        _)))
  (return 0))