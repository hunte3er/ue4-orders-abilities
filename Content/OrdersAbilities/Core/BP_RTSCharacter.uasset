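; RTS unit character Blueprint that adds an attribute-driven healthbar on top of its parent class behaviour.
; On BeginPlay it runs the parent logic, then creates an attribute bar widget bound to its health and max health attributes and assigns it to the Healthbar component.
; Tick is empty, and the unconnected gameplay-effect count print and player-owner call never run.
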(event EventBeginPlay
  (|CallParentFunction)
  (CallFunction|CreateHealthbar))

(event EventTick
  (params (DeltaSeconds :type Float%20%28single-precision%29)))

(fn ConstructionScript)

(fn CreateHealthbar
  (bind _returnvalue (UserInterface|CreateWidget "/FPGameplayAbilities/Widgets/WBP_FPGAAttributeBar.WBP_FPGAAttributeBar_C" 0 self "(R=0.750000,G=0.000000,B=0.000000,A=1.000000)" "(R=0.000000,G=0.750000,B=0.000000,A=1.000000)" (LocalVariables|GetHealthAttribute) (LocalVariables|GetMaxHealthAttribute)))
  (UserInterface|SetWidget (Variables|Default|GetHealthbar) _returnvalue))