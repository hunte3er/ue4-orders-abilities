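; Basic attack ability for RTS units that, given a valid event target, plays the unit's attack montage.
; It looks up the montage in DT_UnitAnimations by the ability system component's name, scaling play rate from AttackSpeed and montage length.
; AttackSpeed also serves as the cooldown and the delay before the ability ends.
; Montage notifies feed an empty OnNotifyBegin hook, also called directly when no row is found.
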(event Custom|OnNotifyBegin
  (params (NotifyName :type Name)))

(event Ability|EventActivateAbilityFromEvent
  (params (EventData :type Gameplay%20Event%20Data%20Structure%20%28by%20ref%29))
  (bind _returnvalue (Ability|GetAbilitySystemComponentfromActorInfo))
  (bind _attackspeedattribute (Variables|Default|GetAttackSpeedAttribute))
  (bind _returnvalue_2 (Ability|Attribute|GetFloatAttributefromAbilitySystemComponent _returnvalue _attackspeedattribute))
  (Utilities|IsValid (.Target (Utilities|Struct|BreakGameplayEventData EventData))
    (:Is%20Valid
      (bind _returnvalue_3 (Utilities|GetDataTableRow "/Game/MyGame/Units/DT_UnitAnimations.DT_UnitAnimations" (Class|RTSAbilitySystemComponent|GetName (.AsRTSAbility%20System%20Component (Utilities|Casting|CastToRTSAbilitySystemComponent (Ability|GetAbilitySystemComponent (Ability|GetOwningActorfromActorInfo))))))
        (:then
          (bind _returnvalue_4 (Animation|GetPlayLength (.AttackMontage (Utilities|Struct|BreakUnitAnimationRow _returnvalue_3))))
          (Utilities|FlowControl|Sequence
            (:then_0
              (Ability|Tasks|WaitDelay _returnvalue_2
                (:OnFinish
                  (Ability|EndAbility))))
            (:then_1
              (bind _notifyname (|PlayMontageandWaitProxy "PlayMontageNotify" (.AttackMontage (Utilities|Struct|BreakUnitAnimationRow _returnvalue_3)) (* (/ _returnvalue_2 _returnvalue_4) 0.5) "None" true false 1.0)
                (:OnNotifyBegin
                  (CallFunction|OnNotifyBegin _notifyname))))))
        (:RowNotFound
          (Development|PrintString "Attack montage not found")
          (CallFunction|OnNotifyBegin "None")
          (Ability|EndAbility))))
    (:Is%20Not%20Valid
      (Development|PrintString "Not valid"))))

(fn GetAbilityCooldown
  (params (AbilitySystem :type Ability%20System%20Component%20Object%20Reference))
  (return (.ReturnValue (Ability|Attribute|GetFloatAttributefromAbilitySystemComponent AbilitySystem (Variables|Default|GetAttackSpeedAttribute)))))