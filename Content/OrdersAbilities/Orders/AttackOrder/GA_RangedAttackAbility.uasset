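; Gameplay Ability for a ranged attack order, which fires a projectile at the target carried by the current event data.
; When a notify begins, it sends the Event.Attack.Ranged gameplay event to the owning actor and gets the spawn transform from that actor.
; It spawns the configured projectile class, handing it the target data, the owner's ability system and an outgoing effect spec built from TestGameplayEffect.
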(event EventOnNotifyBegin
  (params (NotifyName :type Name :default "None"))
  (Ability|SendGameplayEventtoActor (Ability|GetOwningActorfromActorInfo) "(TagName=\"Event.Attack.Ranged\")" (Variables|Default|GetCurrentEventData))
  (bind _returnvalue (Class|ProjectileInterface|GetProjectileSpawn(Message) (Ability|GetOwningActorfromActorInfo)))
  (Game|SpawnActorfromClass (Variables|Default|GetProjectileClass) _returnvalue "Undefined" 0 (Ability|TargetData|AbilityTargetDatafromActor (Utilities|Struct|BreakGameplayEventData (Variables|Default|GetCurrentEventData))) (Ability|GetAbilitySystemComponentfromActorInfo) (Ability|MakeOutgoingGameplayEffectSpec "/Game/MyGame/Units/Snake/TestGameplayEffect.TestGameplayEffect_C") 0))