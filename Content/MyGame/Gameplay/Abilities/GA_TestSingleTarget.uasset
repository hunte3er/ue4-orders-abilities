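; Test gameplay ability that deals single-target damage to the owning AI's current order target.
; It plays the mage attack montage and, on the notify begin, commits the ability.
; If the commit succeeds, it reads the order target from the AI controller's blackboard, applies the test damage effect to it and ends.
; No other path, such as a failed commit, ends the ability.
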(event Ability|EventActivateAbility
  (|PlayMontageandWaitProxy "PlayMontageNotify" "/Game/MyGame/Units/Mage/Montage_Mage_Attack.Montage_Mage_Attack" 1.0 "None" true false 1.0
    (:OnNotifyBegin
      (bind _returnvalue (Ability|CommitAbility))
      (if _returnvalue
        (Utilities|FlowControl|Sequence
          (:then_0
            (GameplayEffects|ApplyGameplayEffectToTarget (Ability|TargetData|AbilityTargetDatafromActor (Class|RTSBlackboardHelper|GetBlackboardOrderTarget (AI|GetBlackboard (AI|GetAIController (Ability|GetOwningActorfromActorInfo))))) "/Game/MyGame/Gameplay/Abilities/GE_TestDamage.GE_TestDamage_C" 1 1))
          (:then_1
            (Ability|EndAbility)))))))