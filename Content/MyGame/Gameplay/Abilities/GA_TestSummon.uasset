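; GA_TestSummon is a gameplay ability that summons a BP_Wasp unit for the owning player, apparently as a test.
; On activation it commits the ability, then asks the RTS game mode to spawn the wasp for the player controller found through the owner's RTSOwnerComponent.
; The spawn point is the AI controller's blackboard order location, raised slightly above it.
; The ability ends afterwards, or immediately if the commit fails.
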(event Ability|EventActivateAbility
  (bind _returnvalue (Ability|CommitAbility))
  (if _returnvalue
    (bind _asrtsgame_mode (Utilities|Casting|CastToRTSGameMode (Game|GetGameMode)))
    (Class|RTSGameMode|SpawnActorforPlayer _asrtsgame_mode "/Game/MyGame/Units/Wasp/BP_Wasp.BP_Wasp_C" (.AsPlayer%20Controller (Utilities|Casting|CastToPlayerController (Components|GetOwner (Class|RTSOwnerComponent|GetPlayerOwner (Actor|GetComponentbyClass (Ability|GetOwningActorfromActorInfo) "/Script/OrdersAbilities.RTSOwnerComponent"))))) (Math|Transform|MakeTransform (+ (Class|RTSBlackboardHelper|GetBlackboardOrderLocation (AI|GetBlackboard (AI|GetAIController (Ability|GetOwningActorfromActorInfo)))) "0, 0,100.000000") "0, 0, 0" "1,1,1"))
    (Ability|EndAbility)
    (else
      (Ability|EndAbility))))