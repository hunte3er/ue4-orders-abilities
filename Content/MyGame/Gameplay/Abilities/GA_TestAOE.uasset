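; GA_TestAOE is a test area-of-effect damage Gameplay Ability targeted at the AI's blackboard order location.
; Activation prints the ability level and plays the Wasp attack montage.
; On notify begin, a successful commit draws a debug sphere, overlaps Pawns in that radius and applies GE_TestDamage at the ability's level.
; The ability then ends; no other montage outcome ends it.
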(event Ability|EventActivateAbility
  (bind _returnvalue (Math|Float|MakeLiteralFloat 5e+02))
  (bind _returnvalue_2 (Ability|GetOwningActorfromActorInfo))
  (bind _returnvalue_3 (AI|GetAIController _returnvalue_2))
  (bind _returnvalue_4 (AI|GetBlackboard _returnvalue_3))
  (bind _returnvalue_5 (Class|RTSBlackboardHelper|GetBlackboardOrderLocation _returnvalue_4))
  (Development|PrintString (Utilities|String|ToString(Integer) (Ability|GetAbilityLevel)))
  (|PlayMontageandWaitProxy "PlayMontageNotify" "/Game/MyGame/Units/Wasp/Montage_Wasp_Attack.Montage_Wasp_Attack" 1.0 "None" true false 1.0
    (:OnNotifyBegin
      (Utilities|FlowControl|Sequence
        (:then_0
          (bind _returnvalue_6 (Ability|CommitAbility))
          (if _returnvalue_6
            (Rendering|Debug|DrawDebugSphere _returnvalue_5 _returnvalue 12 "(R=1.000000,G=1.000000,B=1.000000,A=1.000000)" 1.0)
            (bind _outactors (Collision|SphereOverlapActors _returnvalue_5 _returnvalue (Utilities|Array|MakeArray "ObjectTypeQuery3") 0))
            (GameplayEffects|ApplyGameplayEffectToTarget (Ability|TargetData|AbilityTargetDatafromActorArray _outactors) "/Game/MyGame/Gameplay/Abilities/GE_TestDamage.GE_TestDamage_C" (Ability|GetAbilityLevel) 1)))
        (:then_1
          (Ability|EndAbility))))))