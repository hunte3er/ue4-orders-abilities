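; BP_Projectile is a homing projectile that delivers a Gameplay Ability System effect to its target.
; On server Tick, it refreshes the location of the first actor in its TargetData and moves straight toward it at ProjectileSpeed.
; Within a small radius, it applies the GameplayEffect spec to a valid target's ability system and destroys itself.
; An acceleration-based steering event, ApplyCrappyPhysics, exists but is not called here.
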(event Custom|ApplyCrappyPhysics
  (Variables|Default|SetAcceleration (* (Math|Vector|Normalize (- (Variables|Default|GetTargetLocation) (Transformation|GetActorLocation))) (* (Variables|Default|GetProjectileSpeed) 5.0)))
  (Variables|Default|SetVelocity (* (Math|Vector|Normalize (+ (Variables|Default|GetVelocity) (* (Variables|Default|GetAcceleration) (Utilities|Time|GetWorldDeltaSeconds)))) (Math|Float|Min(Float) (Math|Vector|VectorLength (+ (Variables|Default|GetVelocity) (* (Variables|Default|GetAcceleration) (Utilities|Time|GetWorldDeltaSeconds)))) (Variables|Default|GetProjectileSpeed))))
  (Transformation|AddActorWorldOffset (* (Variables|Default|GetVelocity) (Utilities|Time|GetWorldDeltaSeconds))))

(event Custom|MoveTo
  (Transformation|AddActorWorldOffset (* (Math|Vector|Normalize (- (Variables|Default|GetTargetLocation) (Transformation|GetActorLocation))) (* (Variables|Default|GetProjectileSpeed) (Utilities|Time|GetWorldDeltaSeconds)))))

(event EventTick
  (params (DeltaSeconds :type Float%20%28single-precision%29))
  (bind _targetdata (Variables|Default|GetTargetData))
  (bind _returnvalue (Ability|TargetData|GetActorsfromTargetData _targetdata))
  (bind _output (Utilities|Array|Get(acopy) _returnvalue))
  (Networking|SwitchHasAuthority
    (:Authority
      (CallFunction|SetTargetLocation)
      (if (< (Math|Vector|VectorLength (- (Variables|Default|GetTargetLocation) (Transformation|GetActorLocation))) 1e+02)
        (Utilities|IsValid _output
          (:Is%20Valid
            (GameplayEffects|ApplyGameplayEffectSpecToTarget (Variables|Default|GetAbilitySystem) (Variables|Default|GetGameplayEffect) (Ability|GetAbilitySystemComponent _output))
            (Actor|DestroyActor)))
        (else
          (CallFunction|Moveto))))))

(event EventBeginPlay
  (Variables|Default|SetVelocity (* (Math|Rotator|GetRotationXVector (Transformation|GetActorRotation)) (Variables|Default|GetProjectileSpeed))))

(fn ConstructionScript)

(fn SetTargetLocation
  (bind _targetdata (Variables|Default|GetTargetData))
  (bind _returnvalue (Ability|TargetData|GetActorsfromTargetData _targetdata))
  (bind _output (Utilities|Array|Get(acopy) _returnvalue))
  (bind _returnvalue_2 (Transformation|GetActorLocation _output))
  (Utilities|IsValid _output
    (:Is%20Valid
      (Variables|Default|SetTargetLocation _returnvalue_2)
      (return _returnvalue_2))))